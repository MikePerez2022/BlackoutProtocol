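; Health pickup for the horror shooter that restores a fixed amount of HP when an actor overlaps it.
; The overlap event runs the parent handler, then adds to the Character reference's CurrentHP, clamping it at a hardcoded maximum.
; The heal does not check the overlapping actor, and this graph neither sets the Character reference nor destroys the pickup.
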(event `self.ReceiveActorBeginOverlap`
  (params (OtherActor :type "Actor Object Reference"))
  (bind _character (`self.Character`))
  (bind _returnvalue (+ (`ShooterCharacter.CurrentHP` _character) 25.0))
  (`parent.ReceiveActorBeginOverlap` OtherActor)
  (if (> _returnvalue 500.0)
    (set `ShooterCharacter.CurrentHP` 500.0 _character)
    (else
      (set `ShooterCharacter.CurrentHP` _returnvalue _character))))

(fn `UserConstructionScript`
  (`parent.UserConstructionScript`))