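; BP_AmmoPickup is a pickup that, despite its ammo name, recharges the character's flashlight battery on overlap in a horror shooter.
; It runs the parent overlap logic, then adds a fixed amount to the Character reference's Battery, capped at full.
; The new level is passed to DrainLight on the weapon's flashlight, with no check of the overlapping actor in this Blueprint.
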(event `self.ReceiveActorBeginOverlap`
  (params (OtherActor :type "Actor Object Reference"))
  (bind _character (`self.Character`))
  (bind _battery (`ShooterCharacter.Battery` _character))
  (bind _returnvalue (+ _battery 15.0))
  (`parent.ReceiveActorBeginOverlap` OtherActor)
  (if (> _returnvalue 100.0)
    (`ShooterCharacter.SetBattery` _character 100.0)
    (else
      (`ShooterCharacter.SetBattery` _character _returnvalue)))
  (`FlashlightComponent.DrainLight` (`/Game/Variant_Shooter/Blueprints/Pickups/Weapons/BP_ShooterWeapon_Pistol.Flashlight` (`/Game/HorrorShooter/BP_HSCharacter.Weapon` _character)) _battery))

(fn `UserConstructionScript`
  (`parent.UserConstructionScript`))